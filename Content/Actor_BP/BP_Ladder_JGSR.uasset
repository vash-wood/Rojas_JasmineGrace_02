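; Ladder actor that marks where the adventure player (BP_AdventurePlayer_JGSR) is able to climb.
; On overlap with ClimbVolume, it copies its height and climb speed to the player and sets CanClimbLadder, then clears that flag on exit.
; The climbing itself is not handled here, and debug strings print for any overlapping actor before the player cast.
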(event OnComponentBeginOverlap(ClimbVolume)
  (params (OverlappedComponent :type Primitive%20Component%20Object%20Reference) (OtherActor :type Actor%20Object%20Reference) (OtherComp :type Primitive%20Component%20Object%20Reference) (OtherBodyIndex :type Integer) (bFromSweep :type Boolean) (SweepResult :type Hit%20Result%20Structure%20%28by%20ref%29))
  (Development|PrintString "Can Climb")
  (bind _asbp_adventure_player_jgsr (Utilities|Casting|CastToBP_AdventurePlayer_JGSR OtherActor))
  (Variables|/Game/Game_BP/BP_AdventurePlayer_JGSR.BP_AdventurePlayer_JGSR_C|SetClimbHeight _asbp_adventure_player_jgsr (stale _output_get))
  (Variables|/Game/Game_BP/BP_AdventurePlayer_JGSR.BP_AdventurePlayer_JGSR_C|SetClimbSpeed _asbp_adventure_player_jgsr (Variables|Default|GetLadderClimbSpeed))
  (Variables|/Game/Game_BP/BP_AdventurePlayer_JGSR.BP_AdventurePlayer_JGSR_C|SetCanClimbLadder _asbp_adventure_player_jgsr true))

(event OnComponentEndOverlap(ClimbVolume)
  (params (OverlappedComponent :type Primitive%20Component%20Object%20Reference) (OtherActor :type Actor%20Object%20Reference) (OtherComp :type Primitive%20Component%20Object%20Reference) (OtherBodyIndex :type Integer))
  (Development|PrintString "Can not Climb")
  (bind _asbp_adventure_player_jgsr (Utilities|Casting|CastToBP_AdventurePlayer_JGSR OtherActor))
  (Variables|/Game/Game_BP/BP_AdventurePlayer_JGSR.BP_AdventurePlayer_JGSR_C|SetCanClimbLadder _asbp_adventure_player_jgsr false))

(event EventBeginPlay)

(event Collision|EventActorBeginOverlap
  (params (OtherActor :type Actor%20Object%20Reference)))

(event EventTick
  (params (DeltaSeconds :type Float%20%28single-precision%29)))

(fn ConstructionScript)