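; BP_Water_JGSR is a decal Blueprint that shows a water puddle with a randomly picked texture.
; The construction script creates a dynamic material instance on the decal and sets its puddle texture parameter.
; RandomInteger(2) limits the pick to the first two of four wired textures.
; Random scale and yaw nodes are disconnected and never run, and the event graph is empty.
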(fn `UserConstructionScript`
  ;[1 1 1] setting random texture
  (bind _returnvalue (`DecalComponent.CreateDynamicMaterialInstance` (`self.Decal`)))
  (`MaterialInstanceDynamic.SetTextureParameterValue` _returnvalue "PuddleTexture_" (select `int` (`KismetMathLibrary.RandomInteger` 2) :`0` (`self.Texture_1`) :`1` (`self.Texture_2`) :`2` (`self.Texture_3`) :`3` (`self.Texture_4`))))