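; Fish actor that moves along the spline of a BP_Swim_JGSR actor.
; On BeginPlay it takes the actor returned by GetActorOfClass and starts a timeline with play rate set to the inverse of its completion-time variable.
; Each update maps the timeline value to spline distance and sets the actor transform, using world-space location but local-space rotation.
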(event `self.ReceiveBeginPlay`
  (bind _returnvalue (`GameplayStatics.GetActorOfClass` "/Game/Game_BP/BP_Swim_JGSR.BP_Swim_JGSR_C"))
  (set `self.Spline Ref` _returnvalue)
  (`self.Move Object`))

(event `Move Object`
  (`TimelineComponent.SetPlayRate` (`self.Move Object T`) (/ 1.0 (`self.Time To Comeplete`)))
  (bind (_direction _newtrack_0) (`Timeline|Move Object T`)
    (:`Update`
      (bind _returnvalue (`KismetMathLibrary.Lerp` 0.0 (`SplineComponent.GetSplineLength` (`/Game/Game_BP/BP_Swim_JGSR.Spline` (`self.Spline Ref`))) _newtrack_0))
      (`self.K2_SetActorTransform` (`KismetMathLibrary.MakeTransform` (`SplineComponent.GetLocationAtDistanceAlongSpline` (`/Game/Game_BP/BP_Swim_JGSR.Spline` (`self.Spline Ref`)) _returnvalue "World") (`SplineComponent.GetRotationAtDistanceAlongSpline` (`/Game/Game_BP/BP_Swim_JGSR.Spline` (`self.Spline Ref`)) _returnvalue "Local"))))))

(fn `UserConstructionScript`)