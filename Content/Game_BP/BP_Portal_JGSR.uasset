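; Portal actor that teleports the adventure player to a linked Target portal when they overlap its capsule.
; Before teleporting, it hides the Target, disabling its Niagara effect and CanPort to prevent bounce-back, then after a brief delay calls PortalTo, keeping control rotation.
; When the player leaves a portal's capsule, that portal reactivates.
; The construction script captures the scene through a cube scene capture.
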(event `self.Capsule.OnComponentBeginOverlap`
  (params (OverlappedComponent :type "PrimitiveComponent Object Reference") (OtherActor :type "Actor Object Reference") (OtherComp :type "PrimitiveComponent Object Reference") (OtherBodyIndex :type Integer) (bFromSweep :type Boolean) (SweepResult :type "HitResult Structure (by ref)"))
  (bind _target (`self.Target`))
  (bind _asbp_adventure_player_jgsr (cast `/Game/Game_BP/BP_AdventurePlayer_JGSR` OtherActor))
  (set `self.As BP Adventure Player JGSR_0` _asbp_adventure_player_jgsr)
  (if (`self.Can Port`)
    (`self.HidePortal` _target)
    (`KismetSystemLibrary.Delay` 0.02)
    (`/Game/Game_BP/BP_AdventurePlayer_JGSR.PortalTo` (`self.As BP Adventure Player JGSR_0`) (`SceneComponent.K2_GetComponentLocation` (`Actor.RootComponent` _target)) (`Controller.GetControlRotation` (`GameplayStatics.GetPlayerController` 0)))))

(event `self.Capsule.OnComponentEndOverlap`
  (params (OverlappedComponent :type "PrimitiveComponent Object Reference") (OtherActor :type "Actor Object Reference") (OtherComp :type "PrimitiveComponent Object Reference") (OtherBodyIndex :type Integer))
  (cast `/Game/Game_BP/BP_AdventurePlayer_JGSR` OtherActor)
  (`self.ShowPortal`))

(event `ShowPortal`
  (`ActorComponent.SetActive` (`self.NS_Portal_JGSR`) true true)
  (set `self.Can Port` true))

(event `HidePortal`
  (`ActorComponent.Deactivate` (`self.NS_Portal_JGSR`))
  (set `self.Can Port` false))

(fn `UserConstructionScript`
  (`SceneCaptureComponentCube.CaptureScene` (`self.SceneCaptureComponentCube`)))